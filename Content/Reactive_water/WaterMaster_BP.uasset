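; Reactive water manager that lays out a draggable grid of placeholder tiles in the editor and replaces them with WaterNoSim_BP actors at BeginPlay.
; Two 0.2-second loops swap tiles between WaterSim_BP and WaterNoSim_BP by player distance, limiting simulation to nearby water.
; While the character overlaps the plane collider, Tick records body and leg contact points, velocity-based wave height and beta rain drops, and fires randomly delayed idle-wave dispatchers.
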(event OnComponentBeginOverlap(PlaneCollider)
  (params (OverlappedComponent :type Primitive%20Component%20Object%20Reference) (OtherActor :type Actor%20Object%20Reference) (OtherComp :type Primitive%20Component%20Object%20Reference) (OtherBodyIndex :type Integer) (bFromSweep :type Boolean) (SweepResult :type Hit%20Result%20Structure%20%28by%20ref%29))
  ;[1 1 1] Is Char Overlapping PlaneCollider?
  (if (== OtherComp (Variables|/Game/ThirdPersonBP/Blueprints/ThirdPersonCharacter.ThirdPersonCharacter_C|GetOverlapWaterCheck (Variables|Default|Getcharacter)))
    (Variables|Default|SetCharIsOverlapping true)))

(event OnComponentEndOverlap(PlaneCollider)
  (params (OverlappedComponent :type Primitive%20Component%20Object%20Reference) (OtherActor :type Actor%20Object%20Reference) (OtherComp :type Primitive%20Component%20Object%20Reference) (OtherBodyIndex :type Integer))
  ;[1 1 1] Is Char Overlapping PlaneCollider?
  (if (== OtherComp (Variables|/Game/ThirdPersonBP/Blueprints/ThirdPersonCharacter.ThirdPersonCharacter_C|GetOverlapWaterCheck (Variables|Default|Getcharacter)))
    (Variables|Default|SetCharIsOverlapping false)))

(event EventBeginPlay
  (bind _returnvalue (Game|GetPlayerCharacter 0))
  (Utilities|FlowControl|Sequence
    (:then_0
      ;[1 1 1] Replace Placeholder Tilemeshes with No Water Simulation Blueprint at start
      (for _array_element (Variables|Default|GetPlaceholderTilesArray)
        (Game|SpawnActorfromClass "/Game/Reactive_water/WaterNoSim_BP.WaterNoSim_BP_C" (Transformation|GetWorldTransform _array_element) "Undefined" 0 0)
        (Components|DestroyComponent _array_element)))
    (:then_1
      ;[1 1 1] Set character and max walk speed variable for Idle and velocity based wave height
      (bind _asthird_person_character (Utilities|Casting|CastToThirdPersonCharacter _returnvalue))
      (Variables|Default|Setcharacter _asthird_person_character)
      (Variables|Default|SetCharMaxWalkSpeed (Variables|/Script/Engine.CharacterMovementComponent|GetMaxWalkSpeed (Variables|/Script/Engine.Character|GetCharacterMovement _returnvalue))))
    (:then_2
      ;[1 1 1] Check @ start if Char is overlapping with Base Plane Collider
      (Variables|Default|SetCharIsOverlapping (Class|PrimitiveComponent|IsOverlappingComponent (Variables|/Game/ThirdPersonBP/Blueprints/ThirdPersonCharacter.ThirdPersonCharacter_C|GetOverlapWaterCheck (Variables|Default|Getcharacter)) (Variables|Default|GetPlaneCollider))))
    (:then_3
      ;[1 0.4688 0.4688] Despawn Water Simulation Blueprint and replace wit non simlulation Blueprint
      ;;[1 1 1] Start Distance Check far for despawning SimTiles, then loop
      (bind _outactors (Actor|GetAllActorsOfClass "/Game/Reactive_water/WaterSim_BP.WaterSim_BP_C" :!label _label))
      (for _array_element_2 _outactors
        (if (>= (Math|Vector|VectorLength (- (Transformation|GetWorldLocation (Variables|/Script/Engine.Character|GetCapsuleComponent (Variables|Default|Getcharacter))) (Transformation|GetWorldLocation (Variables|/Game/Reactive_water/WaterSim_BP.WaterSim_BP_C|Getplanecenter _array_element_2)))) (Variables|WaterPlane|GetDeSpawnLastSimTimDist))
          ;;[1 1 1] Spawn NoSimTile at Location of SimPlane and Destroy NoSimTile
          (Game|SpawnActorfromClass "/Game/Reactive_water/WaterNoSim_BP.WaterNoSim_BP_C" (Transformation|GetWorldTransform (Variables|/Script/Engine.StaticMeshActor|GetStaticMeshComponent _array_element_2)) "Undefined" 0 0)
          (Actor|DestroyActor _array_element_2)))
      (Utilities|FlowControl|Delay 0.2)
      (goto _label))
    (:then_4
      ;[0.3719 0.9402 1] Spawn Water Simulation Blueprint and despawn non simulating blueprint
      ;;[1 1 1] Start Distance Check near for spawning SimTiles, then loop
      (bind _outactors_2 (Actor|GetAllActorsOfClass "/Game/Reactive_water/WaterNoSim_BP.WaterNoSim_BP_C" :!label _label_2))
      (for _array_element_3 _outactors_2
        (if (<= (Math|Vector|VectorLength (- (Transformation|GetWorldLocation (Variables|/Script/Engine.Character|GetCapsuleComponent (Variables|Default|Getcharacter))) (Transformation|GetWorldLocation (Variables|/Game/Reactive_water/WaterNoSim_BP.WaterNoSim_BP_C|Getmeshcenter _array_element_3)))) (Variables|WaterPlane|GetSpawnNextSimTilDist))
          ;;[1 1 1] Spawn SimTile at Location of NoSimTile and Destroy NoSimTile
          (Game|SpawnActorfromClass "/Game/Reactive_water/WaterSim_BP.WaterSim_BP_C" (Math|Transform|MakeTransform (.location (Transformation|GetWorldTransform (Variables|/Script/Engine.Actor|GetRootComponent _array_element_3))) (.rotation (Transformation|GetWorldTransform (Variables|/Script/Engine.Actor|GetRootComponent _array_element_3))) (.scale (Transformation|GetWorldTransform (Variables|/Script/Engine.Actor|GetRootComponent _array_element_3)))) "Undefined" 0 0)
          (Actor|DestroyActor _array_element_3)))
      (Utilities|FlowControl|Delay 0.2)
      (goto _label_2))))

(event EventTick
  (params (DeltaSeconds :type Float%20%28single-precision%29))
  (bind _raindistance (Variables|RainEffect|GetRainDistance))
  (bind _character (Variables|Default|Getcharacter))
  (bind _planecollider (Variables|Default|GetPlaneCollider))
  (bind _randomidlewavesmin (Variables|Advanced_Simulation|IdleWaves|GetRandomIdleWavesMin))
  (bind _character_2 (Variables|Default|Getcharacter))
  (bind _enablecalfcollision (Variables|Collision|GetEnableCalfCollision))
  (bind _randomidlewavesmax (Variables|Advanced_Simulation|IdleWaves|GetRandomIdleWavesMax))
  (bind _enablefeetcollision (Variables|Collision|GetEnableFeetCollision))
  (bind _returnvalue (Transformation|GetVelocity _character))
  (bind _capsulecomponent (Variables|/Script/Engine.Character|GetCapsuleComponent _character_2))
  (bind _watercollider_calf_r (Variables|/Game/ThirdPersonBP/Blueprints/ThirdPersonCharacter.ThirdPersonCharacter_C|GetWaterCollider_Calf_R _character_2))
  (bind _watercollider_foot_l (Variables|/Game/ThirdPersonBP/Blueprints/ThirdPersonCharacter.ThirdPersonCharacter_C|GetWaterCollider_Foot_L _character_2))
  (bind _watercollider_foot_r (Variables|/Game/ThirdPersonBP/Blueprints/ThirdPersonCharacter.ThirdPersonCharacter_C|GetWaterCollider_Foot_R _character_2))
  (bind _watercollider_calf_l (Variables|/Game/ThirdPersonBP/Blueprints/ThirdPersonCharacter.ThirdPersonCharacter_C|GetWaterCollider_Calf_L _character_2))
  (bind _returnvalue_2 (Math|Vector|VectorLength _returnvalue))
  ;[1 1 1] Tick event needed for precise calc across tiles
  (if (Variables|Default|GetCharIsOverlapping)
    (Utilities|FlowControl|Sequence
      (:then_0
        ;[1 1 1] Get Location only when BodyParts is overlapping so that waves only happen when touching surface (False sets it to 0 PlanePivot that is out of UV Space)
        (if (not (Variables|Collision|GetDisableAllCollision))
          (if (Variables|Collision|GetUseBodyColliderOnly)
            (if (and (Class|PrimitiveComponent|IsOverlappingComponent _planecollider _capsulecomponent) (Variables|Collision|GetEnableFullBodyCollider)) :!label _label
              ;[1 1 1] get Location of Body, Feet and Calf
              (Variables|Default|SetBodyLoc (Transformation|GetWorldLocation _capsulecomponent) :!label _label_2)
              (elif (Variables|RainEffect|GetActivate%20Rain)
                (goto _label_2)
                (else
                  (Variables|Default|SetBodyLoc "0, 0, 0"))))
            (else
              (Utilities|FlowControl|Sequence
                (:then_0
                  (goto _label))
                (:then_1
                  (if (and (Class|PrimitiveComponent|IsOverlappingComponent _planecollider _watercollider_calf_l) _enablefeetcollision)
                    (Variables|Default|Setcalf_L_loc (Transformation|GetWorldLocation _watercollider_calf_l))
                    (else
                      (Variables|Default|Setcalf_L_loc "0, 0, 0"))))
                (:then_2
                  (if (and _enablefeetcollision (Class|PrimitiveComponent|IsOverlappingComponent _planecollider _watercollider_calf_r))
                    (Variables|Default|Setcalf_R_loc (Transformation|GetWorldLocation _watercollider_calf_r))
                    (else
                      (Variables|Default|Setcalf_R_loc "0, 0, 0"))))
                (:then_3
                  (if (and (Class|PrimitiveComponent|IsOverlappingComponent _planecollider _watercollider_foot_l) _enablecalfcollision)
                    (Variables|Default|Setfoot_L_loc (Transformation|GetWorldLocation _watercollider_foot_l))
                    (else
                      (Variables|Default|Setfoot_L_loc "0, 0, 0"))))
                (:then_4
                  (if (and _enablecalfcollision (Class|PrimitiveComponent|IsOverlappingComponent _planecollider _watercollider_foot_r))
                    (Variables|Default|Setfoot_R_loc (Transformation|GetWorldLocation _watercollider_foot_r))
                    (else
                      (Variables|Default|Setfoot_R_loc "0, 0, 0")))))))))
      (:then_1
        ;[1 1 1] Wave Height by Velocity
        (bind _output_get (Variables|Default|SetIsNOTIdle (>= _returnvalue_2 1.0)))
        (if (and _output_get (Variables|Advanced_Simulation|Heightbyvelocity|GetEnableWavePowerByVelocity))
          (Variables|Default|SetWaveHeightByVelocity_Internal (Math|Float|Clamp(Float) (* (/ _returnvalue_2 (Variables|Default|GetCharMaxWalkSpeed)) (Variables|Advanced_Simulation|Heightbyvelocity|GetHeightByVelocityMulti)) (Variables|Advanced_Simulation|Heightbyvelocity|GetMinHBVHeight)))
          (else
            (Variables|Default|SetWaveHeightByVelocity_Internal 1.0))))
      (:then_2
        (Utilities|FlowControl|Sequence
          (:then_0
            ;[1 1 1] Random IdleWaveDelayCalc and Fire Event via dispatcher to Water Blueprint
            (if (not (Variables|Default|GetIsNOTIdle))
              (if (Variables|Advanced_Simulation|IdleWaves|GetEnableIdleWaves)
                (Utilities|FlowControl|Sequence
                  (:then_0
                    (Utilities|FlowControl|Delay (Math|Conversions|ToFloat(Integer) (Math|Random|RandomIntegerinRange _randomidlewavesmin _randomidlewavesmax)))
                    (Default|CallFireIdleWaveLF))
                  (:then_1
                    (Utilities|FlowControl|Delay (Math|Conversions|ToFloat(Integer) (Math|Random|RandomIntegerinRange _randomidlewavesmin _randomidlewavesmax)))
                    (Default|CallFireIdleWaveRF))
                  (:then_2
                    (Utilities|FlowControl|Delay (Math|Conversions|ToFloat(Integer) (Math|Random|RandomIntegerinRange _randomidlewavesmin _randomidlewavesmax)))
                    (Default|CallFireIdleWaveLC))
                  (:then_3
                    (Utilities|FlowControl|Delay (Math|Conversions|ToFloat(Integer) (Math|Random|RandomIntegerinRange _randomidlewavesmin _randomidlewavesmax)))
                    (Default|CallFireIdleWaveRC))
                  (:then_4
                    (Utilities|FlowControl|Delay (Math|Conversions|ToFloat(Integer) (Math|Random|RandomIntegerinRange _randomidlewavesmin _randomidlewavesmax)))
                    (Default|CallFireIdleWaveBody))))))
          (:then_1
            ;[1 1 1] IdleWaveSize
            (if (Variables|Advanced_Simulation|IdleWaves|GetEnableIdleWaves)
              (if (Variables|Advanced_Simulation|IdleWaves|SmallerIdleWaves|GetEnableSmallerIdleWaves)
                (if (Variables|Default|GetIsNOTIdle)
                  (Utilities|FlowControl|Sequence
                    (:then_0
                      (Variables|Default|SetPawnIdleUpdateRate 1.0)
                      (goto _label_3 Reset))
                    (:then_1
                      (Variables|Default|SetIdle_ForceStrenght_Manipulator 1.0))
                    (:then_2
                      (Variables|Default|SetIdle_ForceSize_Manipulator 1.0)))
                  (else
                    (Utilities|FlowControl|Delay 1.0)
                    (Utilities|FlowControl|DoOnce false :!label _label_3
                      (:Completed
                        (Timeline|Timeline_1 PlayFromStart
                          (:Update
                            (Variables|Default|SetIdle_ForceStrenght_Manipulator (Math|Interpolation|FInterpTo (Variables|Default|GetIdle_ForceStrenght_Manipulator) (Variables|Advanced_Simulation|IdleWaves|SmallerIdleWaves|GetIdleWaveStrenghtMulitplier) (Utilities|Time|GetWorldDeltaSeconds) 1.0))
                            (Variables|Default|SetIdle_ForceSize_Manipulator (Math|Interpolation|FInterpTo (Variables|Default|GetIdle_ForceSize_Manipulator) (Variables|Advanced_Simulation|IdleWaves|SmallerIdleWaves|GetIdleWaveSizeMultiplier) (Utilities|Time|GetWorldDeltaSeconds) 1.0)))))))))))
          (:then_2
            ;[1 1 1] Rain Beta (set rain density with delay + calc random points and convert to vector for use in WaterSim_BP)
            (if (Variables|RainEffect|GetActivate%20Rain)
              (Utilities|FlowControl|Delay (/ 1.0 (Variables|RainEffect|GetRainDensity)))
              (bind _output_get_2 (Variables|Default|SetRandom1 (Math|Random|RandomFloatinRange (* _raindistance -1.0) _raindistance)))
              (bind _output_get_3 (Variables|Default|SetRandom2 (Math|Random|RandomFloatinRange (* _raindistance -1.0) _raindistance)))
              (Variables|Default|SetRainDropLoc (Math|Vector|MakeVector _output_get_2 _output_get_3 0.0)))))))))

(fn ConstructionScript
  ;[1 1 1] Calculate an dragable Array of planes in editor
  (Variables|Default|SetfirstTileLocation (Transformation|GetWorldLocation (Variables|Default|GetStaticMesh)))
  (if (Math|Vector|NotEqual(Vector) (* (Variables|WaterPlane|GetEndPoint) "1.000000,1.000000,0.000000") "0, 0, 0" 0.0001)
    (for _index (range 0 (Math|Float|Floor (/ (.x (Variables|WaterPlane|GetEndPoint)) 1e+03)))
      (for _index_2 (range 0 (Math|Float|Floor (/ (.y (Variables|WaterPlane|GetEndPoint)) 1e+03)))
        ;[1 1 1] Add a static mesh to an array (basically editor usage and visibility of water coverage) + Scale The WaterPlane x2 for better performance/squaremeter
        (bind _returnvalue (AddComponent|AddStaticMeshComponent false (Math|Transform|MakeTransform "0, 0, 0" "0, 0, 0" (Variables|Default|GetMeshScale))))
        (Utilities|Array|AddUnique (Variables|Default|GetPlaceholderTilesArray) _returnvalue)
        (Transformation|AttachComponentToComponent _returnvalue (Variables|Default|GetStaticMesh) "None" "KeepWorld" "KeepRelative" "KeepRelative" true)
        (Transformation|SetRelativeLocation _returnvalue (Math|Vector|MakeVector (* _index 1e+03) (* _index_2 1e+03) 0.0) false false)
        (Variables|WaterPlane|SetEndPoint (Variables|WaterPlane|GetEndPoint))))))

(fn Test)